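; Enemy AI character that chases the player when it sees a pawn and attacks with an axe that knocks back instead of dealing damage.
; PawnSensing triggers an AI MoveTo; on arrival, a CanAttack-gated montage plays with a whoosh, resetting when completed or interrupted.
; The montage notify fires a forward sphere trace that launches any hit Character, adding impact sound, particles and camera shake.
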(event `Chase Player`
  (bind _returnvalue (`self.K2_GetActorLocation`))
  ;[1 1 1] Chase player
  (`|AIMoveTo` self (0.0 0.0 0.0) (`GameplayStatics.GetPlayerCharacter` 0) 120.0
    (:`OnSuccess`
      ;[1 1 1] attack montage
      (if (`self.canAttack?`)
        (`|PlayMontage` (`self.Mesh`) "/Game/Characters/Villagers/Animations/Attack/A_Attack_Montage.A_Attack_Montage"
          (:`then`
            (set `self.canAttack?` false)
            ;[1 1 1] Axe whoosh
            (`GameplayStatics.PlaySoundAtLocation` "/Game/Audio/MS_AxeWhoosh.MS_AxeWhoosh" (`self.K2_GetActorLocation`) (struct) 1.0 1.0 0.0 null null null null))
          (:`OnCompleted`
            (set `self.canAttack?` true :!label _label))
          (:`OnInterrupted`
            (goto _label))
          (:`OnNotifyBegin`
            (bind (_outhit _returnvalue_2) (`KismetSystemLibrary.SphereTraceSingle` :`Start` _returnvalue :`End` (+ _returnvalue (* (`KismetMathLibrary.GetForwardVector` (`self.K2_GetActorRotation`)) 180.0)) :`Radius` 25.0 :`TraceChannel` "TraceTypeQuery3" :`DrawTime` 0.5))
            ;[1 1 1] hit player + sound
            (if _returnvalue_2
              (bind (_bblockinghit _binitialoverlap _time _distance _location _impactpoint _normal _impactnormal _physmat _hitactor) (`GameplayStatics.BreakHitResult` _outhit))
              (bind _ascharacter (cast `Character` _hitactor))
              (`self.LaunchCharacter` _ascharacter (+ (* (`KismetMathLibrary.GetForwardVector` (`self.K2_GetActorRotation`)) (`self.FrontalKnockback`)) (`self.UpwardKnockback`)) false false)
              (`GameplayStatics.PlaySoundAtLocation` "/Game/Audio/MS_AxeHit.MS_AxeHit" (`self.K2_GetActorLocation`) (struct) 1.0 1.0 0.0 null null null null)
              ;[1 1 1] Hit VFX
              (`GameplayStatics.SpawnEmitterAtLocation` "/Game/Realistic_Starter_VFX_Pack_Vol2/Particles/Hit/P_Wood.P_Wood" _impactpoint (`KismetMathLibrary.MakeRotFromX` _normal) (1.5 1.5 1.5))
              ;[1 1 1] camera shake adding
              (`GameplayStatics.PlayWorldCameraShake` "/Game/Blueprints/BP_CameraShake.BP_CameraShake_C" _impactpoint 0.0 1000.0))))))))

(event `self.PawnSensing.OnSeePawn`
  (params (Pawn :type "Pawn Object Reference"))
  ;[1 1 1] Chase player
  (`self.Chase Player`))

(fn `UserConstructionScript`)